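; Slow field actor that drives a gravity-field particle effect and an HP bar widget.
; BeginPlay makes the actor the HP widget's owner, then creates dynamic circle, ring and sparkle materials on the particle component.
; FadeOut restarts a timeline that writes their "Blend" parameter.
; Tick calls FadeOut every frame while RingVisible is true; no slowing or overlap logic is implemented in these graphs.
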(event Custom|FadeOut
  (bind _fade (Timeline|Timeline_0 PlayFromStart)
    (:Update
      (Rendering|Material|SetScalarParameterValue (stale EventBeginPlay _returnvalue) "Blend" _fade :!class /Script/Engine.MaterialInstanceDynamic))))

(event EventBeginPlay
  (bind _gravityps (Variables|Default|GetGravityPS))
  (bind _asgfield_hpbp (Utilities|Casting|CastToGFieldHPBP (UserInterface|GetUserWidgetObject (Variables|Default|GetHPBar))))
  (Variables|/Game/Core/UI/GFieldHPBP.GFieldHPBP_C|SetWidgetOwner _asgfield_hpbp self)
  (Variables|Default|SetAlphaDefault 1.0)
  (bind _returnvalue (Rendering|Material|CreateDynamicMaterialInstance _gravityps 0 "/Game/Core/UI/GravityFieldCircle.GravityFieldCircle" "None" :!class /Script/Engine.PrimitiveComponent))
  (bind _returnvalue_2 (Rendering|Material|CreateDynamicMaterialInstance _gravityps 1 "/Game/Core/UI/GravityFieldRing.GravityFieldRing" "None" :!class /Script/Engine.PrimitiveComponent))
  (bind _returnvalue_3 (Rendering|Material|CreateDynamicMaterialInstance _gravityps 2 "/Game/Core/UI/GravityFieldSparkle.GravityFieldSparkle" "None" :!class /Script/Engine.PrimitiveComponent)))

(event Collision|EventActorBeginOverlap
  (params (OtherActor :type Actor%20Object%20Reference)))

(event EventTick
  (params (DeltaSeconds :type Float%20%28single-precision%29))
  (if (Variables|Default|GetRingVisible)
    (CallFunction|FadeOut)))

(fn ConstructionScript)