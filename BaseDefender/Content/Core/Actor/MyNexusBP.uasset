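; Nexus actor that the player's game is tied to: when it is destroyed, the game returns to the MainMenu level.
; On BeginPlay it links its HP bar widget to itself and registers as a sight stimulus so AI perception can detect it.
; It also sets itself as the ActiveNexus on the player's ThirdPersonCharacter.
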(event EventBeginPlay
  (bind _aiperceptionstimulisource (Variables|Default|GetAIPerceptionStimuliSource))
  (bind _asnexus_hpbp (Utilities|Casting|CastToNexusHPBP (UserInterface|GetUserWidgetObject (Variables|Default|GetHPBar))))
  (Variables|/Game/Core/UI/NexusHPBP.NexusHPBP_C|SetWidgetOwner _asnexus_hpbp self)
  (Class|AIPerceptionStimuliSourceComponent|RegisterforSense _aiperceptionstimulisource "/Script/AIModule.AISense_Sight")
  (Class|AIPerceptionStimuliSourceComponent|RegisterwithPerceptionSystem _aiperceptionstimulisource)
  (bind _asthird_person_character (Utilities|Casting|CastToThirdPersonCharacter (Game|GetPlayerCharacter 0)))
  (Variables|/Game/ThirdPersonCPP/Blueprints/ThirdPersonCharacter.ThirdPersonCharacter_C|SetActiveNexus _asthird_person_character self))

(event Collision|EventActorBeginOverlap
  (params (OtherActor :type Actor%20Object%20Reference)))

(event EventTick
  (params (DeltaSeconds :type Float%20%28single-precision%29)))

(event EventDestroyed
  ;[1 1 1] Nexus de_stroyed
  (Game|OpenLevel(byName) "MainMenu" false))

(fn ConstructionScript)