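; MyTurretBP is a turret actor that carries a health bar widget and an explosion sphere component.
; On BeginPlay it casts the HPBar component's widget to TurretHPBP and sets itself as that widget's owner.
; Every Tick, it checks whether the explosion sphere is visible and, if so, hides it after a 0.4-second delay, so the sphere works as a brief flash.
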(event EventBeginPlay
  (bind _asturret_hpbp (Utilities|Casting|CastToTurretHPBP (UserInterface|GetUserWidgetObject (Variables|Default|GetHPBar))))
  (Variables|/Game/Core/UI/TurretHPBP.TurretHPBP_C|SetWidgetOwner _asturret_hpbp self))

(event Collision|EventActorBeginOverlap
  (params (OtherActor :type Actor%20Object%20Reference)))

(event EventTick
  (params (DeltaSeconds :type Float%20%28single-precision%29))
  (bind _explosionsphere (Variables|Default|GetExplosionSphere))
  (if (Rendering|IsVisible _explosionsphere)
    (Utilities|FlowControl|Delay 0.4)
    (Rendering|SetVisibility _explosionsphere false false)))

(fn ConstructionScript)