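; Minion actor that carries an HP bar widget and holds a debug line-of-sight test against a Turret reference.
; On BeginPlay it casts the HPBar widget to MinionHPBP and sets itself as the widget's owner.
; While the Turret is valid, Tick draws a debug line to its location, runs a Visibility line trace to that point and prints any hit actor and component.
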(event EventBeginPlay
  (bind _asminion_hpbp (Utilities|Casting|CastToMinionHPBP (UserInterface|GetUserWidgetObject (Variables|Default|GetHPBar))))
  (Variables|/Game/Core/UI/MinionHPBP.MinionHPBP_C|SetWidgetOwner _asminion_hpbp self))

(event EventTick
  (params (DeltaSeconds :type Float%20%28single-precision%29))
  (bind _turret (Variables|Default|GetTurret))
  (bind _returnvalue (Transformation|GetActorLocation _turret))
  ;[1 1 1] DrawLine
  (if (Utilities|IsValid _turret)
    (Rendering|Debug|DrawDebugLine "0, 0, 0" _returnvalue "(R=1.000000,G=0.000000,B=0.463735,A=1.000000)" 2.0 4.0)
    (bind (_outhit _returnvalue_2) (Collision|LineTraceByChannel "0, 0, 0" _returnvalue "TraceTypeQuery1" false 0 "None"))
    (if _returnvalue_2
      (Development|PrintString (Utilities|String|BuildString(Object) (Utilities|String|BuildString(Name) "" "" (Utilities|String|StringToName (Utilities|GetDisplayName (.hitactor _outhit))) "hit  ") "" (.hitcomponent _outhit) "comp hit")))))

(fn ConstructionScript)