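; NexusBP is a damageable Nexus actor with an HP component and an HP bar widget.
; BeginPlay adds the HP component and sets itself as the NexusHPBP widget's owner.
; A damage handler removes HP and prints a debug message, but its OnTakeAnyDamage binding sits inside the handler, not in BeginPlay.
; TriggerRanger overlap events are empty, and the mesh play-rate logic is disconnected.
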(event OnComponentBeginOverlap(TriggerRanger)
  (params (OverlappedComponent :type Primitive%20Component%20Object%20Reference) (OtherActor :type Actor%20Object%20Reference) (OtherComp :type Primitive%20Component%20Object%20Reference) (OtherBodyIndex :type Integer) (bFromSweep :type Boolean) (SweepResult :type Hit%20Result%20Structure%20%28by%20ref%29)))

(event OnComponentEndOverlap(TriggerRanger)
  (params (OverlappedComponent :type Primitive%20Component%20Object%20Reference) (OtherActor :type Actor%20Object%20Reference) (OtherComp :type Primitive%20Component%20Object%20Reference) (OtherBodyIndex :type Integer)))

(event Custom|OnTakeAnyDamage_Event_0
  (params (DamagedActor :type Actor%20Object%20Reference) (Damage :type Float%20%28single-precision%29) (DamageType :type Damage%20Type%20Object%20Reference) (InstigatedBy :type Controller%20Object%20Reference) (DamageCauser :type Actor%20Object%20Reference))
  (EventDispatchers|AssignOnTakeAnyDamage (delegate Custom|OnTakeAnyDamage_Event_0))
  (Class|HPComponent|RemoveHP (Variables|Default|GetHPComp) Damage)
  (Development|PrintString "NEXUS DAMAGED"))

(event Collision|EventActorBeginOverlap
  (params (OtherActor :type Actor%20Object%20Reference)))

(event EventTick
  (params (DeltaSeconds :type Float%20%28single-precision%29)))

(event EventBeginPlay
  (bind _returnvalue (AddComponent|AddHPComponent))
  (Variables|Default|SetHPComp _returnvalue)
  (bind _asnexus_hpbp (Utilities|Casting|CastToNexusHPBP (UserInterface|GetUserWidgetObject (Variables|Default|GetHPBar))))
  (Variables|/Game/Core/UI/NexusHPBP.NexusHPBP_C|SetWidgetOwner _asnexus_hpbp self))

(fn ConstructionScript)